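; Frog is a hittable target actor that awards a point when a VehicleAdvPawn runs into it.
; The first vehicle overlap clears a one-shot flag, enables physics on the Cube and launches it upward with a random sideways impulse.
; It plays a hit sound, then after short delays plays a frog noise, calls PointIncrease on VehicleAdvGameMode and later destroys itself.
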(event EventBeginPlay
  (Variables|Components|SetcanIncreaseScore true))

(event Collision|EventActorBeginOverlap
  (params (OtherActor :type Actor%20Object%20Reference))
  (bind _returnvalue (Math|Random|RandomFloatinRange -2e+03 2e+03))
  (bind _returnvalue_2 (Transformation|GetActorLocation))
  (bind _cube (Variables|Default|GetCube))
  (if (Utilities|ClassIsChildOf (Utilities|GetClass OtherActor) "/Game/VehicleTemplate/Blueprints/VehicleAdvPawn.VehicleAdvPawn_C")
    (bind _asvehicle_adv_game_mode (Utilities|Casting|CastToVehicleAdvGameMode (Game|GetGameMode)))
    (if (Variables|Components|GetcanIncreaseScore)
      (Variables|Components|SetcanIncreaseScore false)
      (Physics|SetSimulatePhysics _cube true)
      (Physics|AddImpulseatLocation _cube (Math|Vector|MakeVector _returnvalue _returnvalue 2e+03) _returnvalue_2 "None")
      (Audio|PlaySoundatLocation "/Game/Sound/frogHit_Cue.frogHit_Cue" _returnvalue_2 "0, 0, 0" 1.0 1.0 0.0 0 0 0 0)
      (Utilities|FlowControl|Delay 0.2)
      (Audio|PlaySoundatLocation "/Game/Sound/frog_noise_Cue.frog_noise_Cue" _returnvalue_2 "0, 0, 0" 1.0 1.0 0.0 0 0 0 0)
      (Default|PointIncrease _asvehicle_adv_game_mode)
      (Utilities|FlowControl|Delay 5.0)
      (Actor|DestroyActor))))

(fn ConstructionScript)
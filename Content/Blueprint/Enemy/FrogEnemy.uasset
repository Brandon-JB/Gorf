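; FrogEnemy is an AI-controlled enemy that ends the game when it touches the player's vehicle.
; Shortly after spawning, it writes the VehicleAdvPawn into its blackboard's Player key, and its mesh spins every tick.
; Overlapping the vehicle plays an explosion, calls EndGame on the game mode and opens the GameOver level after a brief delay.
; Overlapping a Wall_BP or another FrogEnemy destroys it.
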(event EventBeginPlay
  (bind _self self)
  (bind _returnvalue (AI|GetAIController _self))
  (bind _returnvalue_2 (AI|GetBlackboard _returnvalue))
  (Utilities|FlowControl|Delay 0.2)
  (bind _returnvalue_3 (Actor|GetActorOfClass "/Game/VehicleTemplate/Blueprints/VehicleAdvPawn.VehicleAdvPawn_C"))
  (Utilities|IsValid _returnvalue_2
    (:Is%20Valid
      (AI|Components|Blackboard|SetValueasObject _returnvalue_2 (Utilities|Name|MakeLiteralName "Player") _returnvalue_3))
    (:Is%20Not%20Valid
      (Development|PrintString "beands"))))

(event Collision|EventActorBeginOverlap
  (params (OtherActor :type Actor%20Object%20Reference))
  (bind _returnvalue (Utilities|GetClass OtherActor))
  (bind _returnvalue_2 (Transformation|GetActorLocation OtherActor))
  (if (Utilities|ClassIsChildOf _returnvalue "/Game/VehicleTemplate/Blueprints/VehicleAdvPawn.VehicleAdvPawn_C")
    (Effects|SpawnEmitteratLocation "/Game/StarterContent/Particles/P_Explosion.P_Explosion" _returnvalue_2 "0, 0, 0" (* (Transformation|GetActorScale3D OtherActor) "5.000000,5.000000,5.000000"))
    (Audio|PlaySoundatLocation "/Game/StarterContent/Audio/Explosion_Cue.Explosion_Cue" _returnvalue_2 "0, 0, 0" 1.0 1.0 0.0 0 0 0 0)
    (bind _asvehicle_adv_game_mode (Utilities|Casting|CastToVehicleAdvGameMode (Game|GetGameMode)))
    (Default|EndGame _asvehicle_adv_game_mode)
    (Utilities|FlowControl|Delay 0.175)
    (Game|OpenLevel(byObjectReference) "/Game/Levels/GameOver.GameOver")
    (elif (or (Utilities|ClassIsChildOf _returnvalue "/Game/Blueprint/Wall_BP.Wall_BP_C") (Utilities|ClassIsChildOf _returnvalue "FrogEnemy_C"))
      (Actor|DestroyActor))))

(event EventTick
  (params (DeltaSeconds :type Float%20%28single-precision%29))
  (Transformation|AddLocalRotation (Variables|Default|GetStaticMesh) "0.000000,0.000000,5.000000" false false))

(fn ConstructionScript)